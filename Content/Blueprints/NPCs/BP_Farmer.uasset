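; Farmer NPC that the player can chat with through a dialogue speaker component system.
; ChatToNpc starts an owned dialogue between its BPCCRPGSpeakerComponent and the target's DialogueSpeakerComponent, if the target has one.
; A W_Dialogue widget built at BeginPlay appears when the player enters NPCRad, then is removed after a short delay or on exit.
; CheckIfAlive is a helper that tests for positive health, unused in these graphs.
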(event `ChatToNpc`
  (params (Target :type "Actor Object Reference"))
  (bind _returnvalue (`self.GetComponentByClass` Target "/Script/DialogueTreeRuntime.DialogueSpeakerComponent"))
  (bind _bpc_crpgspeakercomponent (`self.BPC_CRPGSpeakerComponent`))
  ;[1 1 1] Chat with NPC
  (`/Engine/EditorBlueprintResources/StandardMacros.IsValid` _returnvalue
    (:`Is Valid`
      (`DialogueSpeakerComponent.StartOwnedDialogue` _bpc_crpgspeakercomponent (`|MakeArray` _bpc_crpgspeakercomponent _returnvalue :!type "DialogueSpeakerComponent Object Reference")))))

(event `self.ReceiveBeginPlay`
  ;[1 1 1] Chat with NPC
  (bind _returnvalue (`|GenericCreateObject` "/Game/WidgetsUI/W_Dialogue.W_Dialogue_C"))
  (set `self.CreateInteract` _returnvalue))

(event `self.NPCRad.OnComponentBeginOverlap`
  (params (OverlappedComponent :type "PrimitiveComponent Object Reference") (OtherActor :type "Actor Object Reference") (OtherComp :type "PrimitiveComponent Object Reference") (OtherBodyIndex :type Integer) (bFromSweep :type Boolean) (SweepResult :type "HitResult Structure (by ref)"))
  (bind _createinteract (`self.CreateInteract`))
  ;[1 1 1] Chat with NPC
  (if (== OtherActor (`GameplayStatics.GetPlayerCharacter` 0))
    (`UserWidget.AddToViewport` _createinteract 0)
    (`KismetSystemLibrary.Delay` 3.0)
    (`Widget.RemoveFromParent` _createinteract :!label _label)))

(event `self.NPCRad.OnComponentEndOverlap`
  (params (OverlappedComponent :type "PrimitiveComponent Object Reference") (OtherActor :type "Actor Object Reference") (OtherComp :type "PrimitiveComponent Object Reference") (OtherBodyIndex :type Integer))
  ;[1 1 1] Chat with NPC
  (if (== (`GameplayStatics.GetPlayerCharacter` 0) OtherActor)
    (goto _label)))

(fn `CheckIfAlive`
  (params (Health :type "Float (double-precision)"))
  (returns (IsAlive :type Boolean))
  (return (> Health 0.0)))

(fn `UserConstructionScript`)