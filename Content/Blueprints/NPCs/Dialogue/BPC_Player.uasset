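; Player component that tracks whether six NPCs (Steve, Winston, Terrorbringer, Eugene, Gale, Francis) have registered a win.
; On BeginPlay it starts a self-re-arming one-second timer event for each unchecked NPC, which finds that actor by class and reads its win variable.
; A win sets the matching Time and Check variables, otherwise a debug message prints.
; The timers are never cleared, so polling continues after a win.
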(event `self.ReceiveBeginPlay`
  (`|ExecutionSequence`
    (:`then_0`
      (if (not (`self.CheckSteve`))
        (`self.SteveWin`)))
    (:`then_1`
      (if (not (`self.CheckWinston`))
        (`self.WinstonWin`)))
    (:`then_2`
      (if (not (`self.CheckTerror`))
        (`self.TerrorWin`)))
    (:`then_3`
      (if (not (`self.CheckEugene`))
        (`self.EugeneWin`)))
    (:`then_4`
      (if (not (`self.CheckGale`))
        (`self.GaleWin`)))
    (:`then_5`
      (if (not (`self.CheckFrancis`))
        (`self.FrancisWin`)))))

(event `SteveWin`
  ;[1 1 1] Steve Event
  (`KismetSystemLibrary.K2_SetTimerDelegate` (delegate `SteveWin`) 1.0 true)
  (bind _returnvalue (`GameplayStatics.GetActorOfClass` "/Game/LupeContent/Blueprints/BP_LazySteve.BP_LazySteve_C"))
  (if (== (`/Game/LupeContent/Blueprints/BP_LazySteve.SteveWin?` _returnvalue) 1)
    (set `self.SteveTime` 1)
    (set `self.CheckSteve` true)
    (else
      (`KismetSystemLibrary.PrintString` "STEVE NO WIN"))))

(event `WinstonWin`
  ;[1 1 1] Winston Event
  (`KismetSystemLibrary.K2_SetTimerDelegate` (delegate `WinstonWin`) 1.0 true)
  (bind _returnvalue (`GameplayStatics.GetActorOfClass` "/Game/LupeContent/Blueprints/BP_Winston.BP_Winston_C"))
  (if (== (`/Game/LupeContent/Blueprints/BP_Winston.WinstonWin?` _returnvalue) 1)
    (set `self.WinstonTime` 1)
    (set `self.CheckWinston` true)
    (else
      (`KismetSystemLibrary.PrintString` "WINSTON NO WIN"))))

(event `TerrorWin`
  ;[1 1 1] Terrorbringer Event
  (`KismetSystemLibrary.K2_SetTimerDelegate` (delegate `TerrorWin`) 1.0 true)
  (bind _returnvalue (`GameplayStatics.GetActorOfClass` "/Game/LupeContent/Blueprints/BP_TerrorBringer.BP_TerrorBringer_C"))
  (if (== (`/Game/LupeContent/Blueprints/BP_TerrorBringer.TerrorWin?` _returnvalue) 1)
    (set `self.TerrorTime` 1)
    (set `self.CheckTerror` true)
    (else
      (`KismetSystemLibrary.PrintString` "TERROR NO WIN"))))

(event `EugeneWin`
  ;[1 1 1] Eugene Event
  (`KismetSystemLibrary.K2_SetTimerDelegate` (delegate `EugeneWin`) 1.0 true)
  (bind _returnvalue (`GameplayStatics.GetActorOfClass` "/Game/LupeContent/Blueprints/BP_Eugene.BP_Eugene_C"))
  (if (== (`/Game/LupeContent/Blueprints/BP_Eugene.EugeneWin?` _returnvalue) 1)
    (set `self.EugeneTime` 1)
    (set `self.CheckEugene` true)
    (else
      (`KismetSystemLibrary.PrintString` "EUGENE NO WIN"))))

(event `GaleWin`
  ;[1 1 1] Gale Event
  (`KismetSystemLibrary.K2_SetTimerDelegate` (delegate `GaleWin`) 1.0 true)
  (bind _returnvalue (`GameplayStatics.GetActorOfClass` "/Game/LupeContent/Blueprints/BP_Gale.BP_Gale_C"))
  (if (== (`/Game/LupeContent/Blueprints/BP_Gale.GaleWin?` _returnvalue) 1)
    (set `self.GaleTime` 1)
    (set `self.CheckGale` true)
    (else
      (`KismetSystemLibrary.PrintString` "GALE NO WIN"))))

(event `FrancisWin`
  ;[1 1 1] Francis Event
  (`KismetSystemLibrary.K2_SetTimerDelegate` (delegate `FrancisWin`) 1.0 true)
  (bind _returnvalue (`GameplayStatics.GetActorOfClass` "/Game/LupeContent/Blueprints/BP_Francis.BP_Francis_C"))
  (if (== (`/Game/LupeContent/Blueprints/BP_Francis.FrancisWin?` _returnvalue) 1)
    (set `self.FrancisTime` 1)
    (set `self.CheckFrancis` true)
    (else
      (`KismetSystemLibrary.PrintString` "FRANCIS NO WIN"))))