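; BP_TheSoulEater is an AI character that chases the player once its PawnSensing component sees a pawn.
; Sighting sets the FollowPlayer flag and fires an event that runs AIMoveTo toward the player character, stopping within an acceptance radius.
; Each successful move re-triggers the follow event, then disables character movement if DragonWin is true.
; A failed move does not retry.
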(event `self.PawnSensing.OnSeePawn`
  (params (Pawn :type "Pawn Object Reference"))
  (set `self.FollowPlayer?` true)
  (`self.Follow Player`))

(event `Follow Player`
  (if (`self.FollowPlayer?`)
    (`|AIMoveTo` self (0.0 0.0 0.0) (`GameplayStatics.GetPlayerCharacter` 0) 200.0
      (:`OnSuccess`
        (`self.Follow Player`)
        (if (`self.DragonWin?`)
          (`CharacterMovementComponent.DisableMovement` (`self.CharacterMovement`)))))))

(fn `UserConstructionScript`)