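; BP_TerrorBringer is an enemy pawn that chases the player once it sees them.
; PawnSensing sets a follow flag and triggers TerrorFollowsPlayer, which runs AI MoveTo toward the player character, stopping within an acceptance radius.
; Each successful move re-calls the follow event to keep the chase going, then disables movement if TerrorWin equals one.
; Failed moves have no handler, and nothing here clears the flag or sets TerrorWin.
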(event `self.PawnSensing.OnSeePawn`
  (params (Pawn :type "Pawn Object Reference"))
  ;[1 1 1] Terrorbringer sees player, then follows
  (set `self.FollowPlayer?` true)
  (`self.Terror Follows Player`))

(event `Terror Follows Player`
  ;[1 1 1] Terrorbringer Follows Player
  (if (`self.FollowPlayer?`)
    (`|AIMoveTo` self (0.0 0.0 0.0) (`GameplayStatics.GetPlayerCharacter` 0) 300.0
      (:`OnSuccess`
        (`self.Terror Follows Player`)
        (if (== (`self.TerrorWin?`) 1)
          (`CharacterMovementComponent.DisableMovement` (`self.CharacterMovement`)))))))

(fn `UserConstructionScript`)