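; BP_LazySteve is an AI character that starts following the player once its PawnSensing component sees a pawn.
; It issues AI MoveTo toward the player character and re-calls itself on each successful arrival to keep following.
; A DoOnce adds an audio component the first time the follow starts.
; After an arrival, movement is disabled if SteveWin equals 1, a value this Blueprint's graphs never set.
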(event `self.PawnSensing.OnSeePawn`
  (params (Pawn :type "Pawn Object Reference"))
  ;[1 1 1] Steve sees player, then follows
  (set `self.FollowPlayer?` true)
  (`self.Steve Follow Player`))

(event `Steve Follow Player`
  ;[1 1 1] Steve Follows Player
  (if (`self.FollowPlayer?`)
    (`|AIMoveTo` self (0.0 0.0 0.0) (`GameplayStatics.GetPlayerCharacter` 0) 200.0
      (:`then`
        (`/Engine/EditorBlueprintResources/StandardMacros.DoOnce` false
          (:`Completed`
            (`AddComponent|NODE_AddAudioComponent-0`))))
      (:`OnSuccess`
        (`self.Steve Follow Player`)
        (if (== (`self.SteveWin?`) 1)
          (`CharacterMovementComponent.DisableMovement` (`self.CharacterMovement`)))))))

(fn `UserConstructionScript`)