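; BP_Francis is a pawn that follows the player once its PawnSensing component spots them.
; Sight sets a follow flag and starts FrancisFollowPlayer, which uses AI MoveTo toward the player character, stopping within an acceptance radius.
; Each successful move re-calls the event to keep following, then disables movement if FrancisWin, not set here, equals 1.
; The EugeneFollowPlayer function is empty.
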(event `self.PawnSensing.OnSeePawn`
  (params (Pawn :type "Pawn Object Reference"))
  ;[1 1 1] Francis sees player, then follows
  (set `self.FollowPlayer?` true)
  (`self.Francis Follow Player`))

(event `Francis Follow Player`
  ;[1 1 1] Francis Follows Player
  (if (`self.FollowPlayer?`)
    (`|AIMoveTo` self (0.0 0.0 0.0) (`GameplayStatics.GetPlayerCharacter` 0) 300.0
      (:`OnSuccess`
        (`self.Francis Follow Player`)
        (if (== (`self.FrancisWin?`) 1)
          (`CharacterMovementComponent.DisableMovement` (`self.CharacterMovement`)))))))

(fn `Eugene Follow Player`)

(fn `UserConstructionScript`)