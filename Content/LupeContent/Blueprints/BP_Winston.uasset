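; BP_Winston is an AI pawn, Winston, that follows the player once it sees them.
; PawnSensing sets FollowPlayer and starts WinstonFollowPlayer, which issues AIMoveTo toward the player character with a loose acceptance radius.
; Each successful move calls the event again to keep following, then disables character movement if WinstonWin equals 1.
; Nothing in this graph sets WinstonWin, clears FollowPlayer or handles a failed move.
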(event `self.PawnSensing.OnSeePawn`
  (params (Pawn :type "Pawn Object Reference"))
  ;[1 1 1] Winston sees player, then follows
  (set `self.FollowPlayer?` true)
  (`self.Winston Follow Player`))

(event `Winston Follow Player`
  ;[1 1 1] Winston Follows Player
  (if (`self.FollowPlayer?`)
    (`|AIMoveTo` self (0.0 0.0 0.0) (`GameplayStatics.GetPlayerCharacter` 0) 300.0
      (:`OnSuccess`
        (`self.Winston Follow Player`)
        (if (== (`self.WinstonWin?`) 1)
          (`CharacterMovementComponent.DisableMovement` (`self.CharacterMovement`)))))))

(fn `UserConstructionScript`)